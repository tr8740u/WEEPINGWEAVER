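; Door actor with a player-proximity flag that decides whether it swings open or shut.
; The third-person character sets CanOpen by entering Box and clears it by ending overlap with Frame, not Box.
; DoorOpenClose prints a debug message and snaps the door's yaw open or closed from that flag; nothing here calls it.
; A DoorSwing timeline for animated rotation exists but is disconnected, so it never runs.
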(event `Key|F`
  (params (Key :type "Key Structure")))

(event `self.Box.OnComponentBeginOverlap`
  (params (OverlappedComponent :type "PrimitiveComponent Object Reference") (OtherActor :type "Actor Object Reference") (OtherComp :type "PrimitiveComponent Object Reference") (OtherBodyIndex :type Integer) (bFromSweep :type Boolean) (SweepResult :type "HitResult Structure (by ref)"))
  (cast `/Game/ThirdPerson/Blueprints/BP_ThirdPersonCharacter` OtherActor)
  (set `self.bCanOpen` true))

(event `self.frame.OnComponentEndOverlap`
  (params (OverlappedComponent :type "PrimitiveComponent Object Reference") (OtherActor :type "Actor Object Reference") (OtherComp :type "PrimitiveComponent Object Reference") (OtherBodyIndex :type Integer))
  (cast `/Game/ThirdPerson/Blueprints/BP_ThirdPersonCharacter` OtherActor)
  (set `self.bCanOpen` false))

(fn `DoorOpenClose`
  (`KismetSystemLibrary.PrintText` "DoorOpenClose")
  (if (`self.bCanOpen`)
    (`SceneComponent.K2_SetRelativeRotation` (`self.door`) (`KismetMathLibrary.MakeRotator` 0.0 0.0 90.0) false false)
    (else
      (`SceneComponent.K2_SetRelativeRotation` (`self.door`) (`KismetMathLibrary.MakeRotator` 0.0 0.0 0.0) false false))))

(fn `UserConstructionScript`)